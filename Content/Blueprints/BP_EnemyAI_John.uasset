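; Enemy AI pawn that chases and attacks the living player on sight, with a camera-facing health bar.
; ChasePlayer issues a move and immediately plays a cooldown-gated attack montage, whose notify sphere-traces to launch and damage hit characters.
; Damage, throttled by a one-second lockout, calls UpdateHP to subtract one HP regardless of amount, ragdolling and destroying the enemy at zero.
; First Tick also calls UpdateHP, costing one HP.
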(event `self.ReceiveBeginPlay`)

(event `ChasePlayer`
  (bind _returnvalue (`self.K2_GetActorLocation`))
  (`|AIMoveTo` self (0.0 0.0 0.0) (`GameplayStatics.GetPlayerCharacter` 0) 10.0
    (:`then`
      (if (`self.canAttack?`)
        (`|PlayMontage` (`self.SkeletalMesh`) "/Game/Characters/John/Anim/A_Attack_Montage.A_Attack_Montage"
          (:`then`
            (set `self.canAttack?` false))
          (:`OnCompleted`
            (set `self.canAttack?` true :!label _label))
          (:`OnInterrupted`
            (goto _label))
          (:`OnNotifyBegin`
            (bind (_outhit _returnvalue_2) (`KismetSystemLibrary.SphereTraceSingle` :`Start` _returnvalue :`End` (+ _returnvalue (* (`KismetMathLibrary.GetForwardVector` (`self.K2_GetActorRotation`)) 150.0)) :`Radius` 25.0 :`TraceChannel` "TraceTypeQuery3" :`DrawDebugType` "ForDuration" :`DrawTime` 0.5))
            (if _returnvalue_2
              (`|ExecutionSequence`
                (:`then_1`
                  (bind _ascharacter (cast `Character` (`.HitActor` (`GameplayStatics.BreakHitResult` _outhit))))
                  (`self.LaunchCharacter` _ascharacter (+ (* (`KismetMathLibrary.GetForwardVector` (`self.K2_GetActorRotation`)) 500.0) (0.0 0.0 300.0)) false false)
                  (`GameplayStatics.ApplyDamage` _ascharacter 1.0))))))))))

(event `self.PawnSensing.OnSeePawn`
  (params (Pawn :type "Pawn Object Reference"))
  ; 看到玩家就要攻擊，但如果玩家死了就不攻擊
  (bind _asbp_third_person_character_john (cast `/Game/ThirdPerson/Blueprints/BP_ThirdPersonCharacter_John` (`GameplayStatics.GetPlayerCharacter` 0)))
  (bind _output_get (set `self.As BP Third Person Character John` _asbp_third_person_character_john))
  (if (`/Game/ThirdPerson/Blueprints/BP_ThirdPersonCharacter_John.isALife` _output_get)
    (if true
      (`self.ChasePlayer`))))

(event `self.ReceiveTick`
  (params (DeltaSeconds :type "Float (single-precision)"))
  (bind _widget_hp (`self.Widget_HP`))
  ; 讓血條面對攝影機
  (if (`self.isLife`)
    (`|ExecutionSequence`
      (:`then_0`
        (`SceneComponent.K2_SetWorldRotation` _widget_hp (`KismetMathLibrary.FindLookAtRotation` (`SceneComponent.K2_GetComponentLocation` _widget_hp) (`SceneComponent.K2_GetComponentLocation` (`PlayerCameraManager.TransformComponent` (`GameplayStatics.GetPlayerCameraManager` 0)))) false false))
      (:`then_1`
        (`/Engine/EditorBlueprintResources/StandardMacros.DoOnce` false
          (:`Completed`
            (`self.UpdateHP`)))))))

(event `self.ReceiveAnyDamage`
  (params (Damage :type "Float (single-precision)") (DamageType :type "DamageType Object Reference") (InstigatedBy :type "Controller Object Reference") (DamageCauser :type "Actor Object Reference"))
  (bind _skeletalmesh (`self.SkeletalMesh`))
  ; 被攻擊後減血
  (`/Engine/EditorBlueprintResources/StandardMacros.DoOnce` false :!label _label_2
    (:`Completed`
      (`self.UpdateHP`)
      (if (<= (`self.enemyHP_Current`) 0.0)
        (set `self.isLife` false)
        (`PrimitiveComponent.SetSimulatePhysics` _skeletalmesh true)
        (`PrimitiveComponent.SetCollisionEnabled` _skeletalmesh "QueryAndPhysics")
        (`KismetSystemLibrary.Delay` 1.0)
        (`self.K2_DestroyActor`)
        (else
          (`KismetSystemLibrary.Delay` 1.0)
          (goto _label_2 :!via `Reset`))))))

(event `UpdateHP`
  ; 更新血條
  (bind _output_get (set `self.enemyHP_Current` (- (`self.enemyHP_Current`) 1.0)))
  (bind _aswbp_health_bar (cast `/Game/Blueprints/WBP_HealthBar` (`WidgetComponent.GetWidget` (`self.Widget_HP`))))
  (set `ProgressBar.Percent` (/ _output_get (`self.enemyHP_Max`)) (`/Game/Blueprints/WBP_HealthBar.HealthBar` _aswbp_health_bar)))

(fn `UserConstructionScript`)